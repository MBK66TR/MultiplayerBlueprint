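; BP_HeroQueen is a playable hero character with axis-driven movement, camera look, aim-down-sights and weapon fire.
; The ADS input sets IsADS locally, and non-authority instances also send it to the server.
; Firing works only while aiming, spawning a muzzle effect, playing a pistol sound and running a debug-drawn line trace from the muzzle socket.
; Firing runs locally without a server call, and the trace result is unused.
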(event `InputAxis|Turn`
  (params (AxisValue :type "Float (single-precision)"))
  (`self.AddControllerYawInput` AxisValue))

(event `InputAxis|MoveForward`
  (params (AxisValue :type "Float (single-precision)"))
  (`self.AddMovementInput` (`self.GetActorForwardVector`) AxisValue))

(event `InputAxis|LookUp`
  (params (AxisValue :type "Float (single-precision)"))
  (`self.AddControllerPitchInput` AxisValue))

(event `InputAxis|MoveRight`
  (params (AxisValue :type "Float (single-precision)"))
  (`self.AddMovementInput` (`self.GetActorRightVector`) AxisValue))

(event `Srv_SetADS`
  (params (isADS :type Boolean))
  (set `self.isADS` isADS))

(event `InputAction|ADS`
  (params (Key :type "Key Structure"))
  (:`Pressed`
    (`/Engine/EditorBlueprintResources/ActorMacros.Switch Has Authority`
      (:`Authority`
        _)
      (:`Remote`
        (`self.Srv_SetADS` true)))
    (set `self.isADS` true))
  (:`Released`
    (`/Engine/EditorBlueprintResources/ActorMacros.Switch Has Authority`
      (:`Authority`
        _)
      (:`Remote`
        (`self.Srv_SetADS` false)))
    (set `self.isADS` false)))

(event `InputAction|FireWeapon`
  (params (Key :type "Key Structure"))
  (bind (_returnvalue_location _returnvalue_rotation) (`KismetMathLibrary.BreakTransform` (`SceneComponent.GetSocketTransform` (`self.WeaponMesh`) "Muzzle" "RTS_World")))
  (:`Pressed`
    (if (`self.isADS`)
      (`NiagaraFunctionLibrary.SpawnSystemAttached` "/Game/Niagara/explo.explo" (`self.WeaponMesh`) "Muzzle" (0.0 0.0 0.0) (struct) "SnapToTarget")
      (`GameplayStatics.PlaySound2D` "/Game/500201__bratish__pistol-fire.500201__bratish__pistol-fire" 1.0 1.0 0.0 null null)
      (`KismetSystemLibrary.LineTraceSingle` :`Start` _returnvalue_location :`End` (+ _returnvalue_location (* (`KismetMathLibrary.GetForwardVector` _returnvalue_rotation) 10000)) :`TraceChannel` "TraceTypeQuery1" :`DrawDebugType` "ForDuration"))))

(fn `UserConstructionScript`)